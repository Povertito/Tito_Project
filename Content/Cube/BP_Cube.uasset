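; Player-controlled physics cube for an obstacle-dodging runner, with score taken from its distance along world X.
; BeginPlay sets game-only input, shows the BPScore widget and starts a looping timer that applies velocity-change impulses forward and sideways from the MoveSideways axis.
; Tick updates Score from the cube's position.
; Hitting an actor tagged "obstacle" stops movement and reloads the current level after a delay.
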(event `self.ReceiveTick`
  (params (DeltaSeconds :type "Float (single-precision)"))
  (bind _returnvalue_x (`KismetMathLibrary.BreakVector` (`SceneComponent.K2_GetComponentLocation` (`self.Cube`))))
  (set `self.Score` (`KismetMathLibrary.FTrunc` (/ _returnvalue_x 100.0))))

(event `self.ReceiveBeginPlay`
  (bind _returnvalue (`GameplayStatics.GetPlayerController` 0))
  (`WidgetBlueprintLibrary.SetInputMode_GameOnly` _returnvalue)
  (set `PlayerController.bShowMouseCursor` false _returnvalue)
  (bind _returnvalue_2 (`|CreateWidget` "/Game/Cube/BPScore.BPScore_C"))
  (`UserWidget.AddToViewport` _returnvalue_2 0)
  (`KismetSystemLibrary.K2_SetTimerDelegate` (delegate `MoveCube`) 0.1 true))

(event `MoveCube`
  (if (`self.CanMove`)
    (`PrimitiveComponent.AddImpulse` (`self.Cube`) (`KismetMathLibrary.MakeVector` (`self.ForwardForce`) (* (stale `InputAxis|MoveSideways` AxisValue) (`self.MoveSidewaysForce`))) "None" true)))

(event `InputAxis|MoveSideways`
  (params (AxisValue :type "Float (single-precision)"))
  (if (`self.CanMove`)
    _))

(event `Restartlevel`
  (`KismetSystemLibrary.Delay` (`self.RestartDelay`) :!label _label)
  (bind _returnvalue (`GameplayStatics.GetCurrentLevelName` true))
  (`GameplayStatics.OpenLevel` (`KismetStringLibrary.Conv_StringToName` _returnvalue)))

(event `self.Cube.OnComponentHit`
  (params (HitComponent :type "PrimitiveComponent Object Reference") (OtherActor :type "Actor Object Reference") (OtherComp :type "PrimitiveComponent Object Reference") (NormalImpulse :type "Vector Structure") (Hit :type "HitResult Structure (by ref)"))
  (if (`self.ActorHasTag` OtherActor "obstacle")
    (set `self.CanMove` false)
    (goto _label)))

(fn `UserConstructionScript`)